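; MyRosettaController is a controller Blueprint that manages the inventory UI.
; The OpenInventory input action toggles the Inventory widget on and off the viewport, creating it on first use and caching it in InventoryWidget.
; A ReloadInventory event casts the cached widget to Inventory and calls LoadInventoryItems, doing nothing if no valid widget exists.
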(event `InputAction|OpenInventory`
  (params (Key :type "Key Structure"))
  (bind _inventorywidget (`self.InventoryWidget`))
  (:`Pressed`
    (`/Engine/EditorBlueprintResources/StandardMacros.IsValid` _inventorywidget
      (:`Is Valid`
        (if (`Widget.IsVisible` _inventorywidget)
          (`Widget.RemoveFromParent` _inventorywidget)
          (else
            (`UserWidget.AddToViewport` (`self.InventoryWidget`) 0 :!label _label))))
      (:`Is Not Valid`
        (bind _returnvalue (`|CreateWidget` "/Game/UI/Inventory/Inventory.Inventory_C"))
        (set `self.InventoryWidget` _returnvalue)
        (goto _label)))))

(event `self.ReloadInventory`
  (bind _inventorywidget (`self.InventoryWidget`))
  (`/Engine/EditorBlueprintResources/StandardMacros.IsValid` _inventorywidget
    (:`Is Valid`
      (bind _asinventory (cast `/Game/UI/Inventory/Inventory` _inventorywidget))
      (`/Game/UI/Inventory/Inventory.LoadInventoryItems` _asinventory))))

(fn `UserConstructionScript`)