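; NPC Blueprint for Jerry, who serves a coconut-collection test quest (InventoryTestQuest) through dialogue callbacks.
; OnDialogueEvent, GetBoolValue and GetIntValue switch on the requested name, though their case branches show as unreachable here.
; Those branches hold the logic to begin or update the quest, remove coconuts from the player's inventory, and report quest completion and item count.
; The event graph holds only disabled default events.
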(event EventBeginPlay
  (|CallParentFunction) ; This node is disabled and will not be called.\nDrag off pins to build functionality.
)

(event Collision|EventActorBeginOverlap
  (params (OtherActor :type Actor%20Object%20Reference))
  (|CallParentFunction OtherActor) ; This node is disabled and will not be called.\nDrag off pins to build functionality.
)

(event EventTick
  (params (DeltaSeconds :type Float%20%28single-precision%29))
  (|CallParentFunction DeltaSeconds) ; This node is disabled and will not be called.\nDrag off pins to build functionality.
)

(fn ConstructionScript
  (|CallParentFunction))

(fn OnDialogueEvent
  (params (EventName :type Name%20%28by%20ref%29 :default "None"))
  (|SwitchDialogueCallbackEvent EventName
    (:Default
      (return false))))

(fn GetBoolValue
  (params (ValueName :type Name%20%28by%20ref%29 :default "None"))
  (|SwitchDialogueCallbackBoolValue ValueName
    (:Default
      (return (stale _returnvalue)))))

(fn GetIntValue
  (params (ValueName :type Name%20%28by%20ref%29 :default "None"))
  (|SwitchDialogueCallbackIntValue ValueName
    (:Default
      (return -1))))

(fn ConcludeQuest
  (Class|QuestStatus|UpdateQuests (Variables|Default|GetQuestStatus) "/Game/Quests/InventoryTest/InputAtoms/IT_HasEnoughCoconuts.IT_HasEnoughCoconuts")
  (return))

(fn GiveConconuts
  (Class|RosettaController|RemoveItemfromInventorybyID (Variables|Default|GetPlayerController) "1" 16)
  (return))

(fn TalktoJerry
  (Class|QuestStatus|BeginQuest (Variables|Default|GetQuestStatus) "/Game/Quests/InventoryTestQuest.InventoryTestQuest")
  (return))