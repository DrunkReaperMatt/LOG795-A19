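; NPC Blueprint for Finn, a dialogue character tied to the intro quest.
; Helper functions begin and update the quest through QuestStatus and fetch the player's compared response as an answer prompt.
; Dialogue callbacks report whether the quest is completed and switch on event names, though the helper calls in that event switch are unreachable as shown.
; The event graph holds only disabled default events.
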(fn `Answer Finn`
  (returns (NewParam :type Boolean))
  (`RosettaCharacter.ResponseResult` (`self.PlayerClass`))
  (bind _returnvalue (`RosettaCharacter.CompareResponse` (`self.PlayerClass`)))
  (bind _output_get (set `self.bAnswerPrompt` _returnvalue))
  (return _output_get))

(fn `Conclude Quest`
  (`QuestStatus.UpdateQuests` (`self.QuestStatus`) "/Game/Quests/Intro/InputAtoms/IQ_AnswerFinn.IQ_AnswerFinn")
  (return))

(fn `GetBoolValue`
  (params (ValueName :type "Name (by ref)"))
  (returns (ReturnValue :type Boolean))
  (`|SwitchDialogueCallbackBoolValue` ValueName
    (:`Default`
      _)
    (:`QuestIsCompleted`
      (bind _returnvalue (`QuestStatus.QuestIsCompleted` (`self.QuestStatus`) "/Game/Quests/IntroQuest.IntroQuest"))))
  (return _returnvalue))

(fn `OnDialogueEvent`
  (params (EventName :type "Name (by ref)"))
  (returns (ReturnValue :type Boolean))
  (`|SwitchDialogueCallbackEvent` EventName
    (:`Default`
      (return false))))

(fn `Talk to Finn`
  (`QuestStatus.BeginQuest` (`self.QuestStatus`) "/Game/Quests/IntroQuest.IntroQuest")
  (`QuestStatus.UpdateQuests` (`self.QuestStatus`) "/Game/Quests/Intro/InputAtoms/IQ_TalkToFinn.IQ_TalkToFinn")
  (return))

(fn `UserConstructionScript`
  (`parent.UserConstructionScript`))