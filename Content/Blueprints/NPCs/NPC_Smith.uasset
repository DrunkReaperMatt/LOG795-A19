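; NPC_Smith is the blacksmith NPC Blueprint that handles dialogue for the Obtain Tools quest.
; Dialogue events begin the quest and advance its talk-to-blacksmith and return-tools steps through QuestStatus.
; GetBoolValue answers dialogue conditions from HasStartedQuest, quest completion and a tool item check in the player's inventory.
; ModifyBoolValue always returns false, as its HasStartedQuest assignment is disconnected and never runs.
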(fn `AskForTools`
  (`QuestStatus.BeginQuest` (`self.QuestStatus`) "/Game/Quests/Main/ObtainTools.ObtainTools")
  (`QuestStatus.UpdateQuests` (`self.QuestStatus`) "/Game/Quests/Main/ObtainTools/InputAtoms/Ot_TalkToBlacksmith.OT_TalkToBlacksmith")
  (return))

(fn `GetBoolValue`
  (params (ValueName :type "Name (by ref)"))
  (returns (ReturnValue :type Boolean))
  (`|SwitchDialogueCallbackBoolValue` ValueName
    (:`Default`
      (return false))
    (:`HasAcceptedQuest`
      (return (`self.HasStartedQuest`)))
    (:`HasCompletedQuest`
      (bind _returnvalue (`QuestStatus.QuestIsCompleted` (`self.QuestStatus`) "/Game/Quests/Main/ObtainTools.ObtainTools"))
      (return _returnvalue))
    (:`HasFoundTools`
      (bind _returnvalue_2 (`RosettaController.HasItemInInventoryByID` (`self.PlayerController`) "3"))
      (return _returnvalue_2))))

(fn `ModifyBoolValue`
  (params (ValueName :type "Name (by ref)") (bNewValue :type Boolean))
  (returns (ReturnValue :type Boolean))
  (`|SwitchDialogueCallbackBoolValue` ValueName
    (:`Default`
      (return false))))

(fn `OnDialogueEvent`
  (params (EventName :type "Name (by ref)"))
  (returns (ReturnValue :type Boolean))
  (`|SwitchDialogueCallbackEvent` EventName
    (:`Default`
      _)
    (:`AskToBorrowTools`
      (`self.AskForTools`))
    (:`ReturnTools`
      (`self.ReturnTools`)))
  (return false))

(fn `ReturnTools`
  (`QuestStatus.UpdateQuests` (`self.QuestStatus`) "/Game/Quests/Main/ObtainTools/InputAtoms/OT_ReturnTools.OT_ReturnTools")
  (return))

(fn `UserConstructionScript`
  (`parent.UserConstructionScript`))