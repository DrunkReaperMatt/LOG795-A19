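; Base NPC actor that picks an Angry, Sad or Happy emote name from a sentiment value and can walk away.
; A box overlap registers it on the Rosetta player character, whose quest status it caches at BeginPlay.
; To leave, it swaps visibility and collision with a linked stand-in NPC driven by NPC_Controller's GoAway.
; After a fixed delay, it snaps to the stand-in's pivot and swaps back.
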(event OnComponentBeginOverlap(Box)
  (params (OverlappedComponent :type Primitive%20Component%20Object%20Reference) (OtherActor :type Actor%20Object%20Reference) (OtherComp :type Primitive%20Component%20Object%20Reference) (OtherBodyIndex :type Integer) (bFromSweep :type Boolean) (SweepResult :type Hit%20Result%20Structure%20%28by%20ref%29))
  (bind _asmy_rosetta_character (Utilities|Casting|CastToMyRosettaCharacter OtherActor))
  (Variables|/Game/Blueprints/MyRosettaCharacter.MyRosettaCharacter_C|SetNPC_BaseRef _asmy_rosetta_character self)
  (Development|PrintString (Utilities|String|ToString(Float) (Variables|Default|GetSentimentValueNPC))))

(event OnComponentEndOverlap(Box)
  (params (OverlappedComponent :type Primitive%20Component%20Object%20Reference) (OtherActor :type Actor%20Object%20Reference) (OtherComp :type Primitive%20Component%20Object%20Reference) (OtherBodyIndex :type Integer))
  (bind _asmy_rosetta_character (Utilities|Casting|CastToMyRosettaCharacter OtherActor))
  (Variables|/Game/Blueprints/MyRosettaCharacter.MyRosettaCharacter_C|SetNPC_BaseRef _asmy_rosetta_character 0))

(event Custom|GoAway)

(event Custom|SetIsNameOfEmote
  (bind _erikasnpcref (Variables|Default|GetErikasNPCRef))
  (bind _sentimentvaluenpc (Variables|Default|GetSentimentValueNPC))
  (bind _shouldnpcgoaway (Variables|Default|GetShouldNPCGoAway))
  (bind _pivot (Variables|/Game/Blueprints/NPC_Character.NPC_Character_C|GetPivot _erikasnpcref))
  (bind _returnvalue (Transformation|GetWorldTransform _pivot))
  (Utilities|FlowControl|Sequence
    (:then_0
      (Development|PrintString (Utilities|String|ToString(Float) (Variables|Default|GetSentimentValueNPC)))
      (if (< _sentimentvaluenpc -0.5)
        (bind _output_get (Variables|Default|SetisNameOfEmote "Angry"))
        (Development|PrintString _output_get)
        (elif (>= _sentimentvaluenpc 0.0)
          (bind _output_get_2 (Variables|Default|SetisNameOfEmote "Happy"))
          (Development|PrintString _output_get_2)
          (else
            (bind _output_get_3 (Variables|Default|SetisNameOfEmote "Sad"))
            (Development|PrintString _output_get_3)))))
    (:then_1
      (Development|PrintString (Utilities|String|ToString(Boolean) _shouldnpcgoaway))
      (if _shouldnpcgoaway
        (Development|PrintString "go away event was called")
        (Collision|SetCollisionResponsetoChannel (Variables|Components|GetSkeletalMesh) "ECC_Pawn" "ECR_Ignore")
        (Utilities|FlowControl|Sequence
          (:then_0
            (Rendering|SetVisibility (Variables|Components|GetSkeletalMesh) false false)
            (Collision|SetCollisionResponsetoChannel (Variables|/Script/Engine.Character|GetCapsuleComponent (Variables|Default|GetErikasNPCRef)) "ECC_Pawn" "ECR_Block")
            (bind _asnpc_controller (Utilities|Casting|CastToNPC_Controller (Pawn|GetController (Variables|Default|GetErikasNPCRef))))
            (Default|GoAway _asnpc_controller)
            (Utilities|FlowControl|Delay 3.0)
            (Components|MoveComponentTo (Variables|Components|GetDefaultSceneRoot) (.location _returnvalue) (.rotation _returnvalue) false false 0.0 false)
            (Collision|SetCollisionResponsetoChannel (Variables|/Script/Engine.Character|GetCapsuleComponent (Variables|Default|GetErikasNPCRef)) "ECC_Pawn" "ECR_Ignore")
            (Collision|SetCollisionResponsetoChannel (Variables|Components|GetSkeletalMesh) "ECC_Pawn" "ECR_Block")
            (Utilities|FlowControl|Sequence
              (:then_0
                (Rendering|SetVisibility (Variables|Components|GetSkeletalMesh) true false))
              (:then_1
                (Rendering|SetVisibility (Variables|/Script/Engine.Character|GetMesh (Variables|Default|GetErikasNPCRef)) false false))))
          (:then_1
            (Rendering|SetVisibility (Variables|/Script/Engine.Character|GetMesh (Variables|Default|GetErikasNPCRef)) true false)))
        (else
          (Development|PrintString "should npc go away = false"))))))

(event EventBeginPlay
  (CallFunction|InitVariables)
  (bind _asmy_rosetta_character (Utilities|Casting|CastToMyRosettaCharacter (Game|GetPlayerCharacter 0)))
  (Variables|Default|SetMyRosettaCharacterRef _asmy_rosetta_character))

(fn ConstructionScript)

(fn InitVariables
  (bind _asmy_rosetta_controller (Utilities|Casting|CastToMyRosettaController (Game|GetPlayerController 0)))
  (Variables|QuestStatus|SetPlayerController _asmy_rosetta_controller)
  (bind _asmy_rosetta_character (Utilities|Casting|CastToMyRosettaCharacter (Game|GetPlayerCharacter 0)))
  (bind _output_get (Variables|QuestStatus|SetPlayerClass _asmy_rosetta_character))
  (Variables|QuestStatus|SetQuestStatus (Variables|/Game/Blueprints/MyRosettaCharacter.MyRosettaCharacter_C|GetQuestStatus _output_get)))