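; Non-playable character that registers itself with the player's MyRosettaCharacter and classifies its sentiment as an emote name.
; A box overlap sets the player's NonPlayerCharacter reference to this NPC and clears it on exit.
; SetIsNameOfEmote maps the sentiment value to Angry, Sad or Happy, with debug prints.
; GoAway is an empty event, and the logic that would forward it to NPC_Controller is disconnected.
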(event `GoAway`)

(event `SetIsNameOfEmote`
  (bind _sentimentvaluenpc (`self.SentimentValueNPC`))
  (`|ExecutionSequence`
    (:`then_0`
      (`KismetSystemLibrary.PrintString` (`KismetStringLibrary.Conv_DoubleToString` (`self.SentimentValueNPC`)))
      (if (< _sentimentvaluenpc -0.5)
        (bind _output_get (set `self.isNameOfEmote` "Angry"))
        (`KismetSystemLibrary.PrintString` _output_get)
        (elif (>= _sentimentvaluenpc 0.0)
          (bind _output_get_2 (set `self.isNameOfEmote` "Happy"))
          (`KismetSystemLibrary.PrintString` _output_get_2)
          (else
            (bind _output_get_3 (set `self.isNameOfEmote` "Sad"))
            (`KismetSystemLibrary.PrintString` _output_get_3)))))))

(event `self.Box.OnComponentBeginOverlap`
  (params (OverlappedComponent :type "PrimitiveComponent Object Reference") (OtherActor :type "Actor Object Reference") (OtherComp :type "PrimitiveComponent Object Reference") (OtherBodyIndex :type Integer) (bFromSweep :type Boolean) (SweepResult :type "HitResult Structure (by ref)"))
  (bind _asmy_rosetta_character (cast `/Game/Blueprints/MyRosettaCharacter` OtherActor))
  (set `/Game/Blueprints/MyRosettaCharacter.NonPlayerCharacter` self _asmy_rosetta_character)
  (`KismetSystemLibrary.PrintString` (`KismetStringLibrary.Conv_DoubleToString` (`self.SentimentValueNPC`))))

(event `self.Box.OnComponentEndOverlap`
  (params (OverlappedComponent :type "PrimitiveComponent Object Reference") (OtherActor :type "Actor Object Reference") (OtherComp :type "PrimitiveComponent Object Reference") (OtherBodyIndex :type Integer))
  (bind _asmy_rosetta_character (cast `/Game/Blueprints/MyRosettaCharacter` OtherActor))
  (set `/Game/Blueprints/MyRosettaCharacter.NonPlayerCharacter` null _asmy_rosetta_character))

(event `self.ReceiveBeginPlay`
  (bind _asmy_rosetta_character (cast `/Game/Blueprints/MyRosettaCharacter` (`GameplayStatics.GetPlayerCharacter` 0)))
  (set `self.MyRosettaCharacterRef` _asmy_rosetta_character))

(fn `UserConstructionScript`)