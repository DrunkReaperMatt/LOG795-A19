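; NPC character Blueprint that registers itself with the player's ThirdPersonCharacter while that player is inside its Trigger volume.
; On overlap begin it sets the player's NpcCharacter to itself and copies the player's NonPlayerCharacter into NonPlayerCharacterRef; overlap end clears both references.
; A GoAway event logs a debug message and forwards the call to the NPC_Controller possessing it.
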(event `self.Trigger.OnComponentBeginOverlap`
  (params (OverlappedComponent :type "PrimitiveComponent Object Reference") (OtherActor :type "Actor Object Reference") (OtherComp :type "PrimitiveComponent Object Reference") (OtherBodyIndex :type Integer) (bFromSweep :type Boolean) (SweepResult :type "HitResult Structure (by ref)"))
  (bind _asthird_person_character (cast `/Game/ThirdPersonCPP/Blueprints/ThirdPersonCharacter` OtherActor))
  (set `self.Non player character ref` (`/Game/ThirdPersonCPP/Blueprints/ThirdPersonCharacter.NonPlayerCharacter` _asthird_person_character))
  (set `/Game/ThirdPersonCPP/Blueprints/ThirdPersonCharacter.npc character` self _asthird_person_character))

(event `self.Trigger.OnComponentEndOverlap`
  (params (OverlappedComponent :type "PrimitiveComponent Object Reference") (OtherActor :type "Actor Object Reference") (OtherComp :type "PrimitiveComponent Object Reference") (OtherBodyIndex :type Integer))
  (bind _asthird_person_character (cast `/Game/ThirdPersonCPP/Blueprints/ThirdPersonCharacter` OtherActor))
  (set `self.Non player character ref` null)
  (set `/Game/ThirdPersonCPP/Blueprints/ThirdPersonCharacter.npc character` null _asthird_person_character))

(event `GoAway`
  (`KismetSystemLibrary.PrintString` "go away event was called")
  (bind _asnpc_controller (cast `/Game/Blueprints/NPC_Controller` (`self.GetController`)))
  (`/Game/Blueprints/NPC_Controller.Go Away` _asnpc_controller))

(fn `UserConstructionScript`
  (`parent.UserConstructionScript`))